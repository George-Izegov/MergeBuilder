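; BP_MergeItem is the merge-field item actor, handling the item's sprite visuals, movement and feedback.
; InitVisual async-loads a container or table-data sprite; dusty or boxed items also get a dynamic material with adjusted saturation and a spiderweb sprite overlay.
; MovetoLocation uses a timeline to lerp position with a distance-scaled Z arc.
; Appearing plays a pop sound with timeline scaling; adding a consumable only plays a sound.
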(event EventPlayAddConsumableAnimation
  (params (Type :type EConsumableParamType%20Enum :default "None"))
  (Audio|PlaySound2D "/Game/Development/Sounds/UI/Item_Sell_Purchase_05.Item_Sell_Purchase_05" 1.0 1.0 0.0 0 0))

(event EventInitVisual
  (bind _basedata (Variables|Default|GetBaseData))
  (bind _sprite (Variables|Default|GetSprite))
  (bind (_isdusty _isinbox) (Utilities|Struct|BreakMergeFieldItem _basedata))
  (bind _returnvalue (Transformation|GetRelativeTransform _sprite))
  (Utilities|FlowControl|Sequence
    (:then_0
      (if (Utilities|Struct|BreakMergeFieldItem (Variables|Default|GetBaseData))
        (bind _object (Utilities|AsyncLoadAsset "/Game/Development/Textures/MergeIcons/Containers/Tex_container_04_Sprite.Tex_container_04_Sprite")
          (:Completed
            (bind _aspaper_sprite (Utilities|Casting|CastToPaperSprite _object))
            (Rendering|Components|Sprite|SetSprite (Variables|Default|GetSprite) _aspaper_sprite)))
        (else
          (bind _object_2 (Utilities|AsyncLoadAsset (.Sprite (Utilities|Struct|BreakMergeItemData (Variables|Default|GetTableData))))
            (:Completed
              (bind _aspaper_sprite_2 (Utilities|Casting|CastToPaperSprite _object_2))
              (Rendering|Components|Sprite|SetSprite (Variables|Default|GetSprite) _aspaper_sprite_2))))))
    (:then_1
      (if (or _isdusty _isinbox)
        (Utilities|FlowControl|Sequence
          (:then_0
            (bind _returnvalue_2 (Rendering|Material|CreateDynamicMaterialInstance (Variables|Default|GetSprite) 0 (Rendering|Material|GetMaterial (Variables|Default|GetSprite) 0) "None" :!class /Script/Engine.PrimitiveComponent))
            (Rendering|Material|SetMaterial (Variables|Default|GetSprite) 0 _returnvalue_2)
            (Rendering|Material|SetScalarParameterValue _returnvalue_2 "Saturation" 0.7 :!class /Script/Engine.MaterialInstanceDynamic))
          (:then_1
            (bind _returnvalue_3 (Game|AddComponentbyClass "/Script/Paper2D.PaperSpriteComponent" false (Math|Transform|MakeTransform (+ (.location _returnvalue) "0.000000,0.000000,1.000000") (.rotation _returnvalue) (.scale _returnvalue))))
            (Transformation|AttachComponentToComponent _returnvalue_3 (Variables|Default|GetRoot) "None" "KeepRelative" "KeepRelative" "KeepRelative" true)
            (bind _object_3 (Utilities|AsyncLoadAsset "/Game/Development/Textures/MergeIcons/T_SpiderWeb_3_Sprite.T_SpiderWeb_3_Sprite")
              (:Completed
                (bind _aspaper_sprite_3 (Utilities|Casting|CastToPaperSprite _object_3))
                (Rendering|Components|Sprite|SetSprite _returnvalue_3 _aspaper_sprite_3)))))))))

(event EventMovetoLocation
  (params (Location :type Vector%20%28by%20ref%29 :default "0, 0, 0"))
  (bind _output_get (Variables|Default|SetStartMoveLocation (Transformation|GetActorLocation)))
  (bind (_direction _alpha _deltaz) (Timeline|MoveTimeLine PlayFromStart)
    (:Update
      (Transformation|SetActorLocation (Math|Vector|MakeVector (.x (Math|Vector|Lerp(Vector) _output_get Location _alpha)) (.y (Math|Vector|Lerp(Vector) _output_get Location _alpha)) (+ (.z (Math|Vector|Lerp(Vector) _output_get Location _alpha)) (* _deltaz (/ (Math|Vector|Distance(Vector) _output_get Location) 16.0)))) false false))))

(event EventPlayAppearingAnimation
  (Utilities|FlowControl|Sequence
    (:then_0
      (Audio|PlaySound2D "/Game/Development/Sounds/UI/Pop_09.Pop_09" 1.0 1.0 0.0 0 0))
    (:then_1
      (bind _scale (Timeline|AppearTimeLine PlayFromStart)
        (:Update
          (Transformation|SetActorScale3D (Math|Conversions|ToVector(Float) _scale)))
        (:Finished
          (Transformation|SetActorScale3D "1.000000,1.000000,1.000000"))))))

(fn ConstructionScript)