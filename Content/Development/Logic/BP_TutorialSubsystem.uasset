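; Tutorial subsystem Blueprint that launches the on-screen widget for the current tutorial step.
; StartTutorialStep switches on TutorialStep to blocking-load the widget class for either the collect-tools or collect-reward step.
; StartWidgetStep creates that widget through the MBBasePlayerController, adds it to the viewport, starts it as a TutorialStepWidget and binds an event to its OnFinished.
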(event Custom|StartWidgetStep
  (params (WidgetClass :type Object%20Class%20Reference))
  (bind _asuser_widget (Utilities|Casting|CastToUserWidgetClass WidgetClass))
  (bind _asmbbase_player_controller (Utilities|Casting|CastToMBBasePlayerController (Class|MBTutorialSubsystem|GetPlayerController)))
  (bind _returnvalue (Class|MBBasePlayerController|CreateUserWidget _asmbbase_player_controller _asuser_widget))
  (bind _astutorial_step_widget (Utilities|Casting|CastToTutorialStepWidget _returnvalue))
  (UserInterface|Viewport|AddtoViewport _astutorial_step_widget 10)
  (Class|TutorialStepWidget|StartStep _astutorial_step_widget)
  (EventDispatchers|BindEventtoOnFinished _astutorial_step_widget (EventDispatchers|CreateEvent :!event NextTutorialStep)))

(event EventStartTutorialStep
  (switch int (Variables|Default|GetTutorialStep)
    (:0
      (bind _returnvalue (Utilities|LoadClassAssetBlocking "/Game/Development/Widgets/Tutorial/CollectTools/W_Tutorial_CollectTools.W_Tutorial_CollectTools_C"))
      (CallFunction|StartWidgetStep _returnvalue))
    (:1
      (bind _returnvalue_2 (Utilities|LoadClassAssetBlocking "/Game/Development/Widgets/Tutorial/CollectTools/W_Tutorial_CollectReward.W_Tutorial_CollectReward_C"))
      (CallFunction|StartWidgetStep _returnvalue_2))))