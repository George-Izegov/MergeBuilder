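; BP_GroundTileActor is a ground tile actor for the city system that displays a cube mesh matching its tile type.
; InitMeshbyType switches on the type (base square, one-sided, two-sided corner or edge, three-sided) to pick the matching mesh asset.
; Each branch loads its asset asynchronously, casts it to a static mesh and applies it to BaseMesh once loading completes.
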(event EventInitMeshbyType
  (params (Type :type EGroundTileType%20Enum :default "BaseSquare"))
  (switch Utilities|FlowControl|Switch|SwitchonEGroundTileType Type
    (:BaseSquare
      (bind _object (Utilities|AsyncLoadAsset "/Game/Development/Models/Ground/BaseGroundCube.BaseGroundCube")
        (:Completed
          (bind _asstatic_mesh (Utilities|Casting|CastToStaticMesh _object))
          (Components|StaticMesh|SetStaticMesh (Variables|Default|GetBaseMesh) _asstatic_mesh))))
    (:OneSided
      (bind _object_2 (Utilities|AsyncLoadAsset "/Game/Development/Models/Ground/OneSideGroundCube.OneSideGroundCube")
        (:Completed
          (bind _asstatic_mesh_2 (Utilities|Casting|CastToStaticMesh _object_2))
          (Components|StaticMesh|SetStaticMesh (Variables|Default|GetBaseMesh) _asstatic_mesh_2))))
    (:TwoSidedCorner
      (bind _object_3 (Utilities|AsyncLoadAsset "/Game/Development/Models/Ground/TwoSideCornerGroundCube.TwoSideCornerGroundCube")
        (:Completed
          (bind _asstatic_mesh_3 (Utilities|Casting|CastToStaticMesh _object_3))
          (Components|StaticMesh|SetStaticMesh (Variables|Default|GetBaseMesh) _asstatic_mesh_3))))
    (:TwoSidedEdge
      (bind _object_4 (Utilities|AsyncLoadAsset "/Game/Development/Models/Ground/TwoSideGroundEdgeCube.TwoSideGroundEdgeCube")
        (:Completed
          (bind _asstatic_mesh_4 (Utilities|Casting|CastToStaticMesh _object_4))
          (Components|StaticMesh|SetStaticMesh (Variables|Default|GetBaseMesh) _asstatic_mesh_4))))
    (:ThreeSided
      (bind _object_5 (Utilities|AsyncLoadAsset "/Game/Development/Models/Ground/ThreeSideGroundCube.ThreeSideGroundCube")
        (:Completed
          (bind _asstatic_mesh_5 (Utilities|Casting|CastToStaticMesh _object_5))
          (Components|StaticMesh|SetStaticMesh (Variables|Default|GetBaseMesh) _asstatic_mesh_5))))))

(fn ConstructionScript)