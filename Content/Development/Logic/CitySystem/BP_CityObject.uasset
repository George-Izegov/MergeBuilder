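; BP_CityObject is an actor for city objects that provides visual states for selection and edit feedback.
; Its functions loop over all StaticMeshComponents, toggling custom depth rendering and writing stencil values that distinguish selected, acceptable and unacceptable states.
; Deselect disables custom depth and clears the stencil.
; The event graph and construction script hold no logic.
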(event EventBeginPlay)

(event Collision|EventActorBeginOverlap
  (params (OtherActor :type Actor%20Object%20Reference)))

(event EventTick
  (params (DeltaSeconds :type Float%20%28single-precision%29)))

(fn ConstructionScript)

(fn SetEditMaterial
  (params (IsAcceptable :type Boolean))
  (if IsAcceptable
    (for _array_element (Actor|GetComponentsByClass "/Script/Engine.StaticMeshComponent")
      (Rendering|SetRenderCustomDepth _array_element true)
      (Rendering|SetCustomDepthStencilValue _array_element 3))
    (else
      (for _array_element_2 (Actor|GetComponentsByClass "/Script/Engine.StaticMeshComponent")
        (Rendering|SetRenderCustomDepth _array_element_2 true)
        (Rendering|SetCustomDepthStencilValue _array_element_2 4)))))

(fn SetSelected
  (for _array_element (Actor|GetComponentsByClass "/Script/Engine.StaticMeshComponent")
    (Rendering|SetRenderCustomDepth _array_element true)
    (Rendering|SetCustomDepthStencilValue _array_element 2)))

(fn Deselect
  (for _array_element (Actor|GetComponentsByClass "/Script/Engine.StaticMeshComponent")
    (Rendering|SetRenderCustomDepth _array_element false)
    (Rendering|SetCustomDepthStencilValue _array_element 0)))