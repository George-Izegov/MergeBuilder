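; BP_Water is an actor in the city system that bobs up and down, presumably as the water surface.
; Every Tick it keeps its X and Y and sets Z from a cosine of game time, oscillating around a fixed base height on a short repeating cycle.
; The motion is computed directly from absolute time, with no timeline or stored state, and the construction script is empty.
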(event EventBeginPlay)

(event Collision|EventActorBeginOverlap
  (params (OtherActor :type Actor%20Object%20Reference)))

(event EventTick
  (params (DeltaSeconds :type Float%20%28single-precision%29))
  (bind _returnvalue (Utilities|Time|GetTimeSeconds))
  (bind _returnvalue_2 (Transformation|GetActorLocation))
  (bind _returnvalue_3 (/ _returnvalue 5.0))
  (Transformation|SetActorLocation (Math|Vector|MakeVector (.x _returnvalue_2) (.y _returnvalue_2) (+ -3e+02 (* (Math|Trig|Cos(Degrees) (* (- _returnvalue_3 (Math|Conversions|ToFloat(Integer) (Math|Float|Truncate _returnvalue_3))) 3.6e+02)) 5e+01))) false false))

(fn ConstructionScript)