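; Shop subsystem Blueprint that handles real-money store products and purchases, implemented only for Google Play on Android.
; It gathers store product IDs from shop data tables and queries their SKU details, setting a short timer if IAP is not initialized.
; Billing results grant rewards for each purchased product and call success or failure notifications.
; The App Store purchase event is an empty stub, and the products-received failure call is never reached.
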(event Custom|SkuResponse
  (params (ResponseCode :type EBillingResponseCode%20Enum :default "BILLING_UNAVAILABLE") (ResponseMessage :type String) (SkuDetailsRecords :type Array%20of%20Sku%20Details%20Record%20Structures))
  (Development|PrintString 0 ResponseMessage)
  (Variables|Default|SetGooglePlayOffers SkuDetailsRecords)
  (Default|CallOnStoreProductsReceivedSuccess))

(event Custom|PurchaseResult
  (params (ResponseCode :type EBillingResponseCode%20Enum :default "BILLING_UNAVAILABLE") (ResponseMessage :type String) (UpdatedPurchaseRecords :type Array%20of%20Purchase%20Record%20Structures))
  (Development|PrintString 0 ResponseMessage)
  (if (Utilities|Enum|Equal(Enum) ResponseCode "OK")
    (for _array_element UpdatedPurchaseRecords
      (Class|ShopSubsystem|GiveRewardOfProduct (Utilities|Struct|BreakPurchaseRecord _array_element)))
    (Default|CallOnPurchaseSuccess (Variables|Default|GetProcessedStoreProductID))
    (else
      (Default|CallOnPurchaseFailed (Variables|Default|GetProcessedStoreProductID)))))

(event EventRequestStoreProductsInfo
  (bind _outrownames (DataTable|GetDataTableRowNames (Variables|Default|GetProductsDataTable)))
  (for _array_element _outrownames
    (bind _returnvalue (Utilities|GetDataTableRow "/Game/Development/DataTables/ShopItems.ShopItems" _array_element)
      (:then
        (if (.IsStoreProduct (Utilities|Struct|BreakProduct _returnvalue))
          (Utilities|Array|Add (Variables|Default|GetStoreProductIDs) (.ProductID (Utilities|Struct|BreakProduct _returnvalue)))))))
  (switch string (Game|GetPlatformName)
    (:Android
      (if (Class|AndroidPlayBillingSubsystem|IsIAPInitialized)
        (Class|AndroidPlayBillingSubsystem|QuerySkuDetails (delegate Custom|SkuResponse) (Variables|Default|GetStoreProductIDs) "INAPP")
        (else
          (Development|PrintString 0 "IAP Not init")
          (Utilities|Time|SetTimerbyEvent (EventDispatchers|CreateEvent :!event RequestStoreProductsInfo) 0.5))))))

(event EventMakeGooglePlayPurchase
  (params (ProductID :type String))
  (bind _output_get (Variables|Default|SetProcessedStoreProductID ProductID))
  (Class|AndroidPlayBillingSubsystem|LaunchBillingFlow (delegate Custom|PurchaseResult) _output_get "INAPP"))

(event EventMakeAppStorePurchase
  (params (ProductID :type String)))